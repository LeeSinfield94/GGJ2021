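; Material crafting station actor that opens a crafting menu when the diver enters its interact box.
; Paired DoOnce gates on overlap toggle input, menu visibility with forward/reverse intro animation, and inventory HUD redraw; a separate event refreshes that HUD's materials.
; Custom-depth stencil marks the mesh, and Tick spins the analyser.
; Helper functions match crystals by type, recolour and reveal placed ones, and blend the camera to the station on the fourth; the tube-raising timer is unwired.
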(event `Refresh Material Inventory`
  (bind _asinventory_hud (cast `/Game/UI/Inventory_HUD` (`WidgetComponent.GetUserWidgetObject` (`self.InventoryHUD`)))
    (:`then`
      (`/Game/UI/Inventory_HUD.Get Materials` _asinventory_hud))
    (:`CastFailed`
      (`KismetSystemLibrary.PrintString` "FAILED CAST"))))

(event `Highlight Crown`)

(event `self.ReceiveTick`
  (params (DeltaSeconds :type "Float (single-precision)"))
  (`SceneComponent.K2_AddWorldRotation` (`self.Analyser_LOC`) (struct :`Yaw` 1.0) false false))

(event `self.ReceiveBeginPlay`
  (bind _cube (`self.Cube`))
  (`PrimitiveComponent.SetRenderCustomDepth` _cube true)
  (`PrimitiveComponent.SetRenderCustomDepth` (`self.SidePart_1`) true)
  (`PrimitiveComponent.SetCustomDepthStencilValue` _cube 2)
  (`PrimitiveComponent.SetCustomDepthStencilValue` (`self.SidePart_1`) 2))

(event `Start Tube Animation`
  (params (Condition :type Boolean))
  (bind _widget1 (`self.Widget1`))
  (if Condition
    (`SceneComponent.SetVisibility` _widget1 true false)
    (else
      (`SceneComponent.SetVisibility` _widget1 false false))))

(event `self.InteractBox.OnComponentBeginOverlap`
  (params (OverlappedComponent :type "PrimitiveComponent Object Reference") (OtherActor :type "Actor Object Reference") (OtherComp :type "PrimitiveComponent Object Reference") (OtherBodyIndex :type Integer) (bFromSweep :type Boolean) (SweepResult :type "HitResult Structure (by ref)"))
  (bind _inventoryhud (`self.InventoryHUD`))
  (bind _ascrafting_menu (cast `/Game/UI/CraftingMenu` (`WidgetComponent.GetUserWidgetObject` (`self.Widget1`)) :!pure true))
  (bind _asdiver_bp (cast `/Game/Blueprints/Diver_BP` OtherActor))
  (`/Engine/EditorBlueprintResources/StandardMacros.DoOnce` false :!label _label
    (:`Completed`
      (set `self.Player` _asdiver_bp)
      (`self.EnableInput` (`GameplayStatics.GetPlayerController` 0))
      (`self.Start Tube Animation` true)
      (set `self.IsOverlapped` true)
      (`/Game/UI/CraftingMenu.IntroAnim` _ascrafting_menu 2.0 "Forward")
      (`WidgetComponent.SetManuallyRedraw` _inventoryhud false)
      (goto _label_2 :!via `Reset`))))

(event `Tube_Animation`
  (`SceneComponent.K2_AddWorldOffset` (`self.SP_Point_1`) (`self.AnimUP`) false false))

(event `self.InteractBox.OnComponentEndOverlap`
  (params (OverlappedComponent :type "PrimitiveComponent Object Reference") (OtherActor :type "Actor Object Reference") (OtherComp :type "PrimitiveComponent Object Reference") (OtherBodyIndex :type Integer))
  (cast `/Game/Blueprints/Diver_BP` OtherActor)
  (`/Engine/EditorBlueprintResources/StandardMacros.DoOnce` false :!label _label_2
    (:`Completed`
      (set `self.Player` null)
      (`self.DisableInput` (`GameplayStatics.GetPlayerController` 0))
      (`self.Start Tube Animation` false)
      (set `self.IsOverlapped` false)
      (`/Game/UI/CraftingMenu.IntroAnim` (cast `/Game/UI/CraftingMenu` (`WidgetComponent.GetUserWidgetObject` (`self.Widget1`)) :!pure true) 2.0 "Reverse")
      (`WidgetComponent.SetManuallyRedraw` (`self.InventoryHUD`) true)
      (goto _label :!via `Reset`))))

(fn `CheckCrystals`
  (params (CrystalNumber :type "/Game/Blueprints/Base_Placing_Crystal Object Reference") (Array :type "Array of /Game/Blueprints/Base_Gemstone Object Reference") (InputPin :type Integer))
  (returns (NewParam :type "/Game/Blueprints/Base_Gemstone Object Reference"))
  (bind _materialinstance (`/Game/Blueprints/Base_Placing_Crystal.MaterialInstance` CrystalNumber))
  (bind _output (`|GetArrayItem` (`self.ChildActorComponents`) InputPin))
  (for _array_element Array
    (`/Engine/EditorBlueprintResources/StandardMacros.IsValid` _array_element
      (:`Is Valid`
        (if (== (`/Game/Blueprints/Base_Placing_Crystal.CrystalType` CrystalNumber) (`/Game/Blueprints/Base_Gemstone.CrystalType` _array_element))
          (`/Engine/EditorBlueprintResources/StandardMacros.IsValid` _output
            (:`Is Valid`
              (`MaterialInstanceDynamic.SetVectorParameterValue` _materialinstance "CrystalColor" (`/Game/Blueprints/Base_Gemstone.Colour` _array_element))
              (`MaterialInstanceDynamic.SetVectorParameterValue` _materialinstance "Glimmer Color" (`/Game/Blueprints/Base_Gemstone.GlimmerColour` _array_element))
              (`SceneComponent.SetVisibility` _output true false)
              (bind _result (`/Engine/EditorBlueprintResources/StandardMacros.IncrementInt` (`self.PlacedCrystals`))
                (:`  `
                  (if (== _result 4)
                    (`PlayerController.SetViewTargetWithBlend` (`GameplayStatics.GetPlayerController` 0) self 4.0 "VTBlend_Linear" 4.0 false)
                    (set `self.IsOverlapped` true)
                    (else
                      (return _array_element))))))))))))

(fn `GetAllCrystals`
  (set `self.ChildActorComponents` (`|MakeArray` null null null null :!type "ChildActorComponent Object Reference")))

(fn `UserConstructionScript`)