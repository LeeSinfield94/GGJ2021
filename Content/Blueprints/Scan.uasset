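; Scan is a short-lived expanding scan pulse actor that highlights crystals it reaches.
; On BeginPlay, a fast looping timer grows the SCANSphere's world scale in small increments, and the actor destroys itself after a two-second delay.
; Overlaps on the Sphere component cast the other actor to Base_Crystal and call its Highlight function.
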(event `self.ReceiveBeginPlay`
  (`KismetSystemLibrary.K2_SetTimerDelegate` (delegate `AddScale`) 0.005 true)
  (`KismetSystemLibrary.RetriggerableDelay` 2.0)
  (`self.K2_DestroyActor`))

(event `AddScale`
  (bind _scan_sphere (`self.SCAN_Sphere`))
  (`SceneComponent.SetWorldScale3D` _scan_sphere (+ (`SceneComponent.K2_GetComponentScale` _scan_sphere) (0.1 0.1 0.1))))

(event `self.Sphere.OnComponentBeginOverlap`
  (params (OverlappedComponent :type "PrimitiveComponent Object Reference") (OtherActor :type "Actor Object Reference") (OtherComp :type "PrimitiveComponent Object Reference") (OtherBodyIndex :type Integer) (bFromSweep :type Boolean) (SweepResult :type "HitResult Structure (by ref)"))
  (bind _asbase_crystal (cast `/Game/Blueprints/Base_Crystal` OtherActor))
  (`/Game/Blueprints/Base_Crystal.Highlight` _asbase_crystal))

(fn `UserConstructionScript`)