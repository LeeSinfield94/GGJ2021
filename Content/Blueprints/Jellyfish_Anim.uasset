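; Jellyfish actor that moves its skeletal mesh along a spline from BeginPlay.
; A timeline, rate-scaled by Ship3SplineDuration, drives an alpha that is lerped over the spline length to set the mesh's world location.
; When the timeline finishes, it is reversed to send the jellyfish back along the path.
; A second timeline and spline branch exists but is never triggered.
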(event `self.ReceiveBeginPlay`
  (`self.JellyfishMove`))

(event `JellyfishMove`
  (`TimelineComponent.SetPlayRate` (`self.Timeline_0`) (/ 1.0 (`self.Ship3SplineDuration`)))
  (bind (_direction _newtrack_0) (`Timeline|Timeline_0` :!label _label)
    (:`Update`
      (set `self.JellyAlpha` _newtrack_0)
      (`SceneComponent.K2_SetWorldLocation` (`self.SkeletalMesh`) (`SplineComponent.GetLocationAtDistanceAlongSpline` (`self.Spline`) (`KismetMathLibrary.Lerp` 0.0 (`SplineComponent.GetSplineLength` (`self.Spline`)) (`self.JellyAlpha`)) "World") false false))
    (:`Finished`
      (`self.Finsih`))))

(event `Finsih`
  (goto _label :!via `Reverse`))

(fn `UserConstructionScript`)