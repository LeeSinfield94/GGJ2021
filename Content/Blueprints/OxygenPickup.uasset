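; Oxygen pickup that raises the oxygen level of the diver who overlaps its capsule, then destroys itself.
; A Highlight event marks it for five seconds through custom depth with a stencil value and plays a sonar beep at the given pitch.
; A retriggerable delay extends the highlight on repeated calls before switching the depth rendering and sound off.
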(event `Highlight`
  (params (PitchMultiplier :type "Float (double-precision)"))
  (bind _e (`self.e`))
  (set `AudioComponent.PitchMultiplier` PitchMultiplier (`self.371178__samsterbirdies__sonar-sweep-beep`))
  (`PrimitiveComponent.SetRenderCustomDepth` _e true)
  (`PrimitiveComponent.SetCustomDepthStencilValue` _e 2)
  (`ActorComponent.SetActive` (`self.371178__samsterbirdies__sonar-sweep-beep`) true false)
  (`KismetSystemLibrary.RetriggerableDelay` 5.0)
  (`PrimitiveComponent.SetRenderCustomDepth` _e false)
  (`PrimitiveComponent.SetCustomDepthStencilValue` _e 0)
  (`ActorComponent.SetActive` (`self.371178__samsterbirdies__sonar-sweep-beep`) false false))

(event `self.Capsule.OnComponentBeginOverlap`
  (params (OverlappedComponent :type "PrimitiveComponent Object Reference") (OtherActor :type "Actor Object Reference") (OtherComp :type "PrimitiveComponent Object Reference") (OtherBodyIndex :type Integer) (bFromSweep :type Boolean) (SweepResult :type "HitResult Structure (by ref)"))
  (bind _asdiver_bp (cast `/Game/Blueprints/Diver_BP` OtherActor))
  (`/Game/Blueprints/Diver_BP.ModifyOxygenLevel` _asdiver_bp true 0.5 true)
  (`self.K2_DestroyActor`))

(fn `UserConstructionScript`)