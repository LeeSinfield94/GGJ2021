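; Intro drop pod actor that carries the diver down through water to a landing zone.
; Tick applies MovementSpeed as vertical offset; water overlap swaps bubble effects and starts a timer ramping descent speed to a cap.
; Landing stops movement, shakes the camera, frees the diver, releases physics doors and spawns Crown_BP for its tube animation.
; An event yaws the rotator, and DropPodState tracks progress on the diver.
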(event `Addturn Rotaiton`
  (params (A :type "Float (double-precision)"))
  (`SceneComponent.K2_AddWorldRotation` (`self.ROTATOR`) (`KismetMathLibrary.MakeRotator` 0.0 0.0 (* A (`self.TurnRateMultiplier`))) false false))

(event `Highlight`
  (params (Pitch :type "Float (double-precision)")))

(event `self.ReceiveTick`
  (params (DeltaSeconds :type "Float (single-precision)"))
  (bind _movementspeed (`self.MovementSpeed`))
  (if (<= _movementspeed 0.0)
    (`self.K2_AddActorWorldOffset` (`KismetMathLibrary.MakeVector` 0.0 0.0 _movementspeed))))

(event `self.ReceiveBeginPlay`
  (bind _cube3 (`self.Cube3`))
  (`PrimitiveComponent.SetRenderCustomDepth` _cube3 true)
  (`PrimitiveComponent.SetRenderCustomDepth` (`self.Cube4`) true)
  (`PrimitiveComponent.SetRenderCustomDepth` (`self.Cube2`) true)
  (`PrimitiveComponent.SetRenderCustomDepth` (`self.Cube1`) true)
  (`PrimitiveComponent.SetCustomDepthStencilValue` _cube3 2)
  (`PrimitiveComponent.SetCustomDepthStencilValue` (`self.Cube4`) 2)
  (`PrimitiveComponent.SetCustomDepthStencilValue` (`self.Cube1`) 2)
  (`PrimitiveComponent.SetCustomDepthStencilValue` (`self.Cube2`) 2)
  (set `/Game/Blueprints/Diver_BP.DropPodState` 1 (cast `/Game/Blueprints/Diver_BP` (`GameplayStatics.GetPlayerCharacter` 0) :!pure true)))

(event `self.Box.OnComponentBeginOverlap`
  (params (OverlappedComponent :type "PrimitiveComponent Object Reference") (OtherActor :type "Actor Object Reference") (OtherComp :type "PrimitiveComponent Object Reference") (OtherBodyIndex :type Integer) (bFromSweep :type Boolean) (SweepResult :type "HitResult Structure (by ref)"))
  (cast `/Game/Blueprints/Water_BP` OtherActor
    (:`then`
      (`/Engine/EditorBlueprintResources/StandardMacros.DoOnce` false
        (:`Completed`
          (bind _returnvalue (`KismetSystemLibrary.K2_SetTimer` null "Speed" 0.05 true))
          (set `self.SpeedTimer` _returnvalue)
          (`SceneComponent.SetVisibility` (`self.Bubbles_3`) true false)
          (`SceneComponent.SetVisibility` (`self.trail`) true false)
          (`SceneComponent.SetVisibility` (`self.Bubbles_4`) false false))))
    (:`CastFailed`
      (cast `/Game/Blueprints/IntroAnimation_Landing_Zone` OtherActor)
      (`/Engine/EditorBlueprintResources/StandardMacros.DoOnce` false
        (:`Completed`
          (`KismetSystemLibrary.K2_ClearAndInvalidateTimerHandle` (`self.SpeedTimer`))
          (set `self.MovementSpeed` 0.0)
          (bind _asdiver_bp (cast `/Game/Blueprints/Diver_BP` (`GameplayStatics.GetPlayerCharacter` 0)))
          (set `/Game/Blueprints/Diver_BP.CanLeavePod` true _asdiver_bp)
          (`GameplayStatics.PlayWorldCameraShake` "/Game/Blueprints/Impact.Impact_C" (`SceneComponent.K2_GetComponentLocation` (`Actor.RootComponent` _asdiver_bp)) 100000.0 100000.0)
          (`KismetSystemLibrary.RetriggerableDelay` 1.0)
          (`self.OpenDoors`)
          (set `/Game/Blueprints/Diver_BP.DropPodState` 2 (cast `/Game/Blueprints/Diver_BP` (`GameplayStatics.GetPlayerCharacter` 0) :!pure true)))))))

(event `OpenDoors`
  (bind _door_1 (`self.Door_1`))
  (`PrimitiveComponent.SetSimulatePhysics` _door_1 true)
  (`PrimitiveComponent.SetSimulatePhysics` (`self.Door_3`) true)
  (`PrimitiveComponent.SetSimulatePhysics` (`self.Door_2`) true)
  (`PrimitiveComponent.SetSimulatePhysics` (`self.Door_4`) true)
  (bind _returnvalue (`|SpawnActorFromClass` "/Game/Blueprints/Crown_BP.Crown_BP_C" (`KismetMathLibrary.MakeTransform` (`SceneComponent.K2_GetComponentLocation` (`self.ROTATOR`))) "Undefined" "OverrideRootScale" null null))
  (`KismetSystemLibrary.RetriggerableDelay` 0.5)
  (`PrimitiveComponent.SetEnableGravity` _door_1 true)
  (`PrimitiveComponent.SetEnableGravity` (`self.Door_2`) true)
  (`PrimitiveComponent.SetEnableGravity` (`self.Door_3`) true)
  (`PrimitiveComponent.SetEnableGravity` (`self.Door_4`) true)
  (`KismetSystemLibrary.RetriggerableDelay` 2.5)
  (`/Game/Blueprints/Crown_BP.Start Tube Animation` _returnvalue))

(fn `Speed`
  (bind _movementspeed (`self.MovementSpeed`))
  (if (<= _movementspeed -10.0)
    (`KismetSystemLibrary.K2_ClearAndInvalidateTimerHandle` (`self.SpeedTimer`))
    (else
      (set `self.MovementSpeed` (- _movementspeed 1.0)))))

(fn `UserConstructionScript`)