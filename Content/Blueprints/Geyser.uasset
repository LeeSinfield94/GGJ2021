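; Geyser actor that pushes the Diver_BP player upward while it is inside the Box volume.
; Begin overlap starts a fast looping timer that feeds upward movement input to the diver, rather than launching it or applying physics force.
; End overlap clears the timer.
; Both overlap handlers pass through a DoOnce with no reset, so the start and stop each fire only once per instance.
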(event `Start Launching`
  (bind _returnvalue (`KismetSystemLibrary.K2_SetTimerDelegate` (delegate `Launch Player`) 0.05 true)))

(event `self.Box.OnComponentBeginOverlap`
  (params (OverlappedComponent :type "PrimitiveComponent Object Reference") (OtherActor :type "Actor Object Reference") (OtherComp :type "PrimitiveComponent Object Reference") (OtherBodyIndex :type Integer) (bFromSweep :type Boolean) (SweepResult :type "HitResult Structure (by ref)"))
  (bind _asdiver_bp (cast `/Game/Blueprints/Diver_BP` OtherActor))
  (`/Engine/EditorBlueprintResources/StandardMacros.DoOnce` false
    (:`Completed`
      (`self.Start Launching`))))

(event `Launch Player`
  (`Pawn.AddMovementInput` (stale `self.Box.OnComponentBeginOverlap` _asdiver_bp) (0.0 0.0 555.0) 1.0 false))

(event `self.Box.OnComponentEndOverlap`
  (params (OverlappedComponent :type "PrimitiveComponent Object Reference") (OtherActor :type "Actor Object Reference") (OtherComp :type "PrimitiveComponent Object Reference") (OtherBodyIndex :type Integer))
  (cast `/Game/Blueprints/Diver_BP` OtherActor)
  (`/Engine/EditorBlueprintResources/StandardMacros.DoOnce` false
    (:`Completed`
      (`KismetSystemLibrary.K2_ClearAndInvalidateTimerHandle` (stale `Start Launching` _returnvalue)))))

(fn `UserConstructionScript`)