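; Inventory Blueprint that tracks crafting material quantities in a map inside a CraftingMaterials variable, along with a settable owner reference.
; AddToInventory and RemoveFromInventory look up an item and write back the adjusted amount, with removal clamped at zero.
; GetValue returns the stored count for a mineral.
; Only existing map keys are accepted; unknown items just print a message and are never added.
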(event `SetOwner`
  (params (MyOwner :type "/Game/Blueprints/Diver_BP Object Reference"))
  (set `self.MyOwner` MyOwner))

(fn `AddToInventory`
  (params (NewItem :type "String (by ref)") (Amount :type Integer))
  (bind _craftingmaterials_craftingmaterials (break `/Game/Blueprints/Crafting_Materials` (`self.CraftingMaterials`)))
  (bind (_value _returnvalue) (`BlueprintMapLibrary.Map_Find` _craftingmaterials_craftingmaterials NewItem))
  (if _returnvalue
    (`BlueprintMapLibrary.Map_Add` _craftingmaterials_craftingmaterials NewItem (+ _value Amount))
    (else
      (`KismetSystemLibrary.PrintString` "THis is not a crafting material"))))

(fn `GetValue`
  (params (Mineral :type String))
  (returns (Value :type Integer))
  (bind _craftingmaterials_craftingmaterials (break `/Game/Blueprints/Crafting_Materials` (`self.CraftingMaterials`)))
  (bind (_value _returnvalue) (`BlueprintMapLibrary.Map_Find` _craftingmaterials_craftingmaterials Mineral))
  (if _returnvalue
    (return _value)
    (else
      (`KismetSystemLibrary.PrintString` "No mineral found."))))

(fn `RemoveFromInventory`
  (params (ItemToFind :type "String (by ref)") (Amount :type Integer))
  (bind _craftingmaterials_craftingmaterials (break `/Game/Blueprints/Crafting_Materials` (`self.CraftingMaterials`)))
  (bind (_value _returnvalue) (`BlueprintMapLibrary.Map_Find` _craftingmaterials_craftingmaterials ItemToFind))
  (bind _returnvalue_2 (- _value Amount))
  (if _returnvalue
    (if (< _returnvalue_2 0)
      (`BlueprintMapLibrary.Map_Add` _craftingmaterials_craftingmaterials ItemToFind 0)
      (else
        (`BlueprintMapLibrary.Map_Add` _craftingmaterials_craftingmaterials ItemToFind _returnvalue_2)))
    (else
      (`KismetSystemLibrary.PrintString` "This is not a crafting material"))))