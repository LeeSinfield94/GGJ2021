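; Crown puzzle actor with four crystal slots that the diver fills from their inventory.
; The interact box toggles input, and pressing Interact class-checks each slot's child actor, though the results are unwired.
; CheckCrystals, uncalled here, matches crystals by type, colours and reveals them, and on the fourth blends the view to the crown.
; Tick then moves the spinning crown along a spline via timeline while the camera tracks it.
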(event `Highlight Crown`)

(event `self.ReceiveBeginPlay`
  (bind _crown (`self.Crown`))
  (`PrimitiveComponent.SetRenderCustomDepth` _crown true)
  (`PrimitiveComponent.SetRenderCustomDepth` (`self.Cube`) true)
  (`PrimitiveComponent.SetRenderCustomDepth` (`self.Tube_4`) true)
  (`PrimitiveComponent.SetRenderCustomDepth` (`self.Tube_3`) true)
  (`PrimitiveComponent.SetRenderCustomDepth` (`self.Tube_2`) true)
  (`PrimitiveComponent.SetRenderCustomDepth` (`self.Tube_1`) true)
  (`PrimitiveComponent.SetCustomDepthStencilValue` _crown 2)
  (`PrimitiveComponent.SetCustomDepthStencilValue` (`self.Cube`) 2)
  (`PrimitiveComponent.SetCustomDepthStencilValue` (`self.Tube_4`) 2)
  (`PrimitiveComponent.SetCustomDepthStencilValue` (`self.Tube_2`) 2)
  (`PrimitiveComponent.SetCustomDepthStencilValue` (`self.Tube_1`) 2)
  (`PrimitiveComponent.SetCustomDepthStencilValue` (`self.Tube_3`) 2)
  (`self.GetAllCrystals`))

(event `Start Tube Animation`
  (bind _returnvalue (`KismetSystemLibrary.K2_SetTimerDelegate` (delegate `Tube_Animation`) 0.01 true))
  (`KismetSystemLibrary.RetriggerableDelay` 1.0)
  (`KismetSystemLibrary.K2_ClearAndInvalidateTimerHandle` _returnvalue))

(event `self.InteractBox.OnComponentBeginOverlap`
  (params (OverlappedComponent :type "PrimitiveComponent Object Reference") (OtherActor :type "Actor Object Reference") (OtherComp :type "PrimitiveComponent Object Reference") (OtherBodyIndex :type Integer) (bFromSweep :type Boolean) (SweepResult :type "HitResult Structure (by ref)"))
  (bind _asdiver_bp (cast `/Game/Blueprints/Diver_BP` OtherActor))
  (`/Engine/EditorBlueprintResources/StandardMacros.DoOnce` false :!label _label
    (:`Completed`
      (set `self.Player` _asdiver_bp)
      (`self.EnableInput` (`GameplayStatics.GetPlayerController` 0))
      (`KismetSystemLibrary.PrintString` "Overlapped")
      (goto _label_2 :!via `Reset`))))

(event `Tube_Animation`
  (`SceneComponent.K2_AddWorldRotation` (`self.Billboard`) (struct :`Pitch` 0.5) false false)
  (`SceneComponent.K2_AddWorldRotation` (`self.Billboard2`) (struct :`Roll` 0.5) false false)
  (`SceneComponent.K2_AddWorldRotation` (`self.Billboard1`) (struct :`Roll` -0.5) false false)
  (`SceneComponent.K2_AddWorldRotation` (`self.Billboard3`) (struct :`Pitch` -0.5) false false))

(event `self.InteractBox.OnComponentEndOverlap`
  (params (OverlappedComponent :type "PrimitiveComponent Object Reference") (OtherActor :type "Actor Object Reference") (OtherComp :type "PrimitiveComponent Object Reference") (OtherBodyIndex :type Integer))
  (cast `/Game/Blueprints/Diver_BP` OtherActor)
  (`/Engine/EditorBlueprintResources/StandardMacros.DoOnce` false :!label _label_2
    (:`Completed`
      (set `self.Player` null)
      (`self.DisableInput` (`GameplayStatics.GetPlayerController` 0))
      (`KismetSystemLibrary.PrintString` "Exited")
      (goto _label :!via `Reset`))))

(event `InputAction|Interact`
  (params (Key :type "Key Structure"))
  (:`Pressed`
    (`KismetSystemLibrary.PrintString` "Interact")
    (if (> (`KismetArrayLibrary.Array_Length` (`/Game/Blueprints/Inventory.Crystals` (`/Game/Blueprints/Diver_BP.Inventory` (`self.Player`)))) 0)
      (for _array_element (`self.ChildActorComponents`)
        (`self.CheckClass` (`ChildActorComponent.ChildActor` _array_element))))))

(event `self.ReceiveTick`
  (params (DeltaSeconds :type "Float (single-precision)"))
  (bind _camera (`self.Camera`))
  (bind _spline (`self.Spline`))
  (bind _crown (`self.Crown`))
  (`SceneComponent.K2_SetWorldRotation` _camera (`KismetMathLibrary.FindLookAtRotation` (`SceneComponent.K2_GetComponentLocation` _camera) (`SceneComponent.K2_GetComponentLocation` (`self.Crown`))) false false)
  (if (`self.Move Up`)
    (bind (_direction _newtrack_0) (`Timeline|SplineLineTime`)
      (:`Update`
        (set `self.CrownAlpha` _newtrack_0)
        (`SceneComponent.K2_SetWorldLocation` _crown (`SplineComponent.GetLocationAtDistanceAlongSpline` _spline (`KismetMathLibrary.Lerp` 0.0 (`SplineComponent.GetSplineLength` _spline) (`self.CrownAlpha`)) "World") false false)
        (`SceneComponent.K2_AddRelativeRotation` _crown (struct :`Yaw` 2.0) false false)))))

(fn `CheckCrystals`
  (params (CrystalNumber :type "/Game/Blueprints/Base_Placing_Crystal Object Reference") (Array :type "Array of /Game/Blueprints/Base_Gemstone Object Reference") (InputPin :type Integer))
  (returns (NewParam :type "/Game/Blueprints/Base_Gemstone Object Reference"))
  (bind _materialinstance (`/Game/Blueprints/Base_Placing_Crystal.MaterialInstance` CrystalNumber))
  (bind _output (`|GetArrayItem` (`self.ChildActorComponents`) InputPin))
  (for _array_element Array
    (`/Engine/EditorBlueprintResources/StandardMacros.IsValid` _array_element
      (:`Is Valid`
        (if (== (`/Game/Blueprints/Base_Placing_Crystal.CrystalType` CrystalNumber) (`/Game/Blueprints/Base_Gemstone.CrystalType` _array_element))
          (`/Engine/EditorBlueprintResources/StandardMacros.IsValid` _output
            (:`Is Valid`
              (`MaterialInstanceDynamic.SetVectorParameterValue` _materialinstance "CrystalColor" (`/Game/Blueprints/Base_Gemstone.Colour` _array_element))
              (`MaterialInstanceDynamic.SetVectorParameterValue` _materialinstance "Glimmer Color" (`/Game/Blueprints/Base_Gemstone.GlimmerColour` _array_element))
              (`SceneComponent.SetVisibility` _output true false)
              (bind _result (`/Engine/EditorBlueprintResources/StandardMacros.IncrementInt` (`self.PlacedCrystals`))
                (:`  `
                  (if (== _result 4)
                    (`PlayerController.SetViewTargetWithBlend` (`GameplayStatics.GetPlayerController` 0) self 4.0 "VTBlend_Linear" 4.0 false)
                    (set `self.Move Up` true)
                    (else
                      (return _array_element))))))))))))

(fn `GetAllCrystals`
  (set `self.ChildActorComponents` (`|MakeArray` (`self.Slot1`) (`self.Slot2`) (`self.Slot3`) (`self.Slot4`))))

(fn `UserConstructionScript`)