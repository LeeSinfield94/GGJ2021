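; Base crystal pickup that the diver collects into their inventory by pressing Interact while inside its interact box, after which it is hidden and its collision disabled.
; Box overlap stores the diver and toggles input on the crystal.
; Highlight briefly enables a custom-depth stencil and sonar beep through a retriggerable delay, and a separate event randomizes roll and yaw.
; The construction script creates a dynamic material for per-instance crystal and glimmer colors.
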(event `Highlight`
  (bind _crystal (`self.Crystal`))
  (`PrimitiveComponent.SetRenderCustomDepth` _crystal true)
  (`PrimitiveComponent.SetCustomDepthStencilValue` _crystal 2)
  (`ActorComponent.SetActive` (`self.371178__samsterbirdies__sonar-sweep-beep`) true false)
  (`KismetSystemLibrary.RetriggerableDelay` 5.0)
  (`PrimitiveComponent.SetRenderCustomDepth` _crystal false)
  (`PrimitiveComponent.SetCustomDepthStencilValue` _crystal 0)
  (`ActorComponent.SetActive` (`self.371178__samsterbirdies__sonar-sweep-beep`) false false))

(event `RandomCrystalRot`
  (bind _returnvalue (`KismetMathLibrary.RandomFloatInRange` 1.0 1000.0))
  (`SceneComponent.K2_SetWorldRotation` (`self.Crystal`) (`KismetMathLibrary.MakeRotator` _returnvalue 0.0 _returnvalue) false false))

(event `InputAction|Interact`
  (params (Key :type "Key Structure"))
  (bind _crystal (`self.Crystal`))
  (:`Pressed`
    (`/Game/Blueprints/Inventory.AddToInventory` (`/Game/Blueprints/Diver_BP.Inventory` (`self.Player`)) self)
    (`PrimitiveComponent.SetCollisionEnabled` (`self.InteractBox`) "NoCollision")
    (`SceneComponent.SetVisibility` _crystal false false)
    (`PrimitiveComponent.SetCollisionEnabled` _crystal "NoCollision")))

(event `self.InteractBox.OnComponentBeginOverlap`
  (params (OverlappedComponent :type "PrimitiveComponent Object Reference") (OtherActor :type "Actor Object Reference") (OtherComp :type "PrimitiveComponent Object Reference") (OtherBodyIndex :type Integer) (bFromSweep :type Boolean) (SweepResult :type "HitResult Structure (by ref)"))
  (bind _asdiver_bp (cast `/Game/Blueprints/Diver_BP` OtherActor))
  (set `self.Player` _asdiver_bp)
  (`self.EnableInput` (`GameplayStatics.GetPlayerController` 0)))

(event `self.InteractBox.OnComponentEndOverlap`
  (params (OverlappedComponent :type "PrimitiveComponent Object Reference") (OtherActor :type "Actor Object Reference") (OtherComp :type "PrimitiveComponent Object Reference") (OtherBodyIndex :type Integer))
  (cast `/Game/Blueprints/Diver_BP` OtherActor)
  (set `self.Player` null)
  (`self.DisableInput` (`GameplayStatics.GetPlayerController` 0)))

(fn `UserConstructionScript`
  (bind _crystal (`self.Crystal`))
  (bind _returnvalue (`PrimitiveComponent.CreateDynamicMaterialInstance` _crystal 0 (`PrimitiveComponent.GetMaterial` _crystal 0) "None"))
  (set `self.MatInstance` _returnvalue)
  (`MaterialInstanceDynamic.SetVectorParameterValue` _returnvalue "CrystalColor" (`self.Colour`))
  (`MaterialInstanceDynamic.SetVectorParameterValue` _returnvalue "Glimmer Color" (`self.GlimmerColour`)))