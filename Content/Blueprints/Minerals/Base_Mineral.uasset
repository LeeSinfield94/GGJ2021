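; Base mineral pickup that the diver collects into their inventory by pressing Interact while inside its InteractBox.
; Overlap stores the Diver_BP and enables input on the actor, and leaving clears both.
; Pickup runs once, adding the mineral's name and amount, spawning a bubble effect, then destroying the actor.
; A random crystal rotation event is included, while material, animation and highlight events are empty stubs.
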(event `LoadMaterialInstance`
  (params (Colour :type "LinearColor Structure") (GlimmerColour :type "LinearColor Structure")))

(event `Play animation`)

(event `RandomCrystalRot`
  (bind _returnvalue (`KismetMathLibrary.RandomFloatInRange` 1.0 1000.0))
  (`SceneComponent.K2_SetWorldRotation` (`self.Base_Rotation`) (`KismetMathLibrary.MakeRotator` _returnvalue 0.0 _returnvalue) false false))

(event `Highlight`
  (params (NewParam :type "Float (double-precision)")))

(event `InputAction|Interact`
  (params (Key :type "Key Structure"))
  (bind _interactbox (`self.InteractBox`))
  (:`Pressed`
    (`/Engine/EditorBlueprintResources/StandardMacros.DoOnce` false
      (:`Completed`
        ;[1 1 1] Comment
        (`/Game/Blueprints/Inventory.AddToInventory` (`/Game/Blueprints/Diver_BP.Inventory` (`self.Player`)) (`self.Mineral Name`) (`self.Add Ammount`))
        (`PrimitiveComponent.SetCollisionEnabled` _interactbox "NoCollision")
        (`GameplayStatics.SpawnEmitterAtLocation` "/Game/Particales/Bubble_Pickup.Bubble_Pickup" (`SceneComponent.K2_GetComponentLocation` _interactbox) (struct) (0.2 0.2 0.2))
        (`KismetSystemLibrary.RetriggerableDelay` 0.1)
        (`self.K2_DestroyActor`)))))

(event `self.InteractBox.OnComponentBeginOverlap`
  (params (OverlappedComponent :type "PrimitiveComponent Object Reference") (OtherActor :type "Actor Object Reference") (OtherComp :type "PrimitiveComponent Object Reference") (OtherBodyIndex :type Integer) (bFromSweep :type Boolean) (SweepResult :type "HitResult Structure (by ref)"))
  ;[1 0 0] Overlap
  (bind _asdiver_bp (cast `/Game/Blueprints/Diver_BP` OtherActor))
  (set `self.Player` _asdiver_bp)
  (`self.EnableInput` (`GameplayStatics.GetPlayerController` 0)))

(event `self.InteractBox.OnComponentEndOverlap`
  (params (OverlappedComponent :type "PrimitiveComponent Object Reference") (OtherActor :type "Actor Object Reference") (OtherComp :type "PrimitiveComponent Object Reference") (OtherBodyIndex :type Integer))
  ;[1 0 0] Overlap
  (cast `/Game/Blueprints/Diver_BP` OtherActor)
  (set `self.Player` null)
  (`self.DisableInput` (`GameplayStatics.GetPlayerController` 0)))

(fn `UserConstructionScript`)